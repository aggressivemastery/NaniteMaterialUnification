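; Demo actor that contrasts a unified material with stand-alone materials on a Nanite static mesh.
; If randomization is on, BeginPlay starts an endless loop with random delays that changes the material and can also swap the mesh.
; Unify mode assigns one shared material and selects its texture through custom primitive data, while the alternative picks from a material array.
; Keys 1 and 2 toggle visibility of stand-alone and unified actors respectively.
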(event Custom|LOOP_MATERIAL_CHANGE
  ;[0.3022 0.3802 0.3491 1 32] ASSIGN UNIFICATION MATERIAL IF ENABLED AND SWAP TEXTURES AT A RANDOM PERIOD
  ;;[1 1 1 1 32] SPREAD WORK (LOOP)
  (Utilities|FlowControl|Delay (Math|Random|RandomFloatinRange 1.0 5.0))
  (if (Variables|Default|GetRANDOMIZE_MESH)
    ;;[1 1 1 1 32] RANDOM NANITE MESH
    (Transformation|SetMobility (Variables|Default|GetNANITE%20MESH) "Movable")
    (Components|StaticMesh|SetStaticMesh (Variables|Default|GetNANITE%20MESH) (.OutItem (Utilities|Array|Random (Variables|Default|GetSTATIC_MESH_ARRAY))))
    (Transformation|SetMobility (Variables|Default|GetNANITE%20MESH) "Static"))
  ;;[1 1 1 1 32] BOOL UNIFY MAT
  (if (Variables|Default|GetUNIFY_MATERIAL)
    ;;[1 1 1 1 32] CHANGE CUSTOM DATA VALUE FOR TEXTURE SELECTION
    (Rendering|Material|SetMaterial (Variables|Default|GetNANITE%20MESH) 0 "/Game/GAMEDEVMICAH_UnifyMaterial/MATERIALS/MAT_CUSTOMDATA.MAT_CUSTOMDATA")
    (Rendering|Material|SetDefaultCustomPrimitiveDataFloat (Variables|Default|GetNANITE%20MESH) 0 (Math|Random|RandomFloatinRange 0.0 (Variables|Default|GetMAX_TEXTURE_INDEX)))
    ;;[1 1 1 1 32] TO LOOP
    (CallFunction|LOOPMATERIALCHANGE)
    (else
      ;;[1 1 1 1 32] SELECT RANDOM MATERIAL
      (Rendering|Material|SetMaterial (Variables|Default|GetNANITE%20MESH) 0 (.OutItem (Utilities|Array|Random (Variables|Default|GetMATERIALS_TEXTURE))))
      (CallFunction|LOOPMATERIALCHANGE))))

(event EventBeginPlay
  ;[1 1 1 1 32] BEGIN PLAY / LOOP
  (if (Variables|Default|GetRANDOMIZE_MAT)
    (CallFunction|LOOPMATERIALCHANGE)))

(event Input|KeyboardEvents|1
  (params (Key :type Key%20Structure :default "None"))
  (bind _nanite_mesh (Variables|Default|GetNANITE%20MESH))
  (bind _returnvalue (Rendering|IsVisible _nanite_mesh))
  ;[0.5501 0.6415 1 1 32] HIDE / UNHIDE BASED ON UNIFY MATERIAL
  (:Pressed
    (if (not (Variables|Default|GetUNIFY_MATERIAL))
      (Rendering|SetVisibility _nanite_mesh (not _returnvalue) false)
      (if _returnvalue
        (Development|PrintString "STAND ALONE MATERALS SHOWN" true false "(R=0.000000,G=0.660000,B=1.000000,A=1.000000)" 1.0)
        (else
          (Development|PrintString "STAND ALONE MATERALS HIDDEN" true false "(R=0.000000,G=0.660000,B=1.000000,A=1.000000)" 1.0))))))

(event Input|KeyboardEvents|2
  (params (Key :type Key%20Structure :default "None"))
  (bind _nanite_mesh (Variables|Default|GetNANITE%20MESH))
  (bind _returnvalue (Rendering|IsVisible _nanite_mesh))
  ;[0.5501 0.6415 1 1 32] HIDE / UNHIDE BASED ON UNIFY MATERIAL
  (:Pressed
    (if (Variables|Default|GetUNIFY_MATERIAL)
      (Rendering|SetVisibility _nanite_mesh (not _returnvalue) false)
      (if _returnvalue
        (Development|PrintString "UNIFIED MATERAL SHOWN" true false "(R=0.000000,G=0.660000,B=1.000000,A=1.000000)" 1.0)
        (else
          (Development|PrintString "UNIFIED  MATERAL HIDDEN" true false "(R=0.000000,G=0.660000,B=1.000000,A=1.000000)" 1.0))))))

(fn ConstructionScript)