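; BP_ISM_ACTORS is an Unify Material demo actor whose instanced static mesh can randomize per-instance material data, with key 2 toggling its visibility and printing the state.
; If RANDOMIZE is set, BeginPlay starts a self-calling event that waits a random few seconds, then writes a random custom data value to each instance.
; A final write after the loop marks the render state dirty, refreshing the batch once per cycle.
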(event Custom|LOOPMATERIALCHANGE
  ;[1 1 1] CHANGE ALL PER INSTANCE DATA TO RANDOM VALUE
  (Utilities|FlowControl|Delay (Math|Random|RandomFloatinRange 1.0 5.0))
  (for _index (range 0 (Components|InstancedStaticMesh|GetInstanceCount (Variables|Default|GetInstancedStaticMesh)))
    (Components|InstancedStaticMesh|SetCustomDataValue (Variables|Default|GetInstancedStaticMesh) _index 0 (Math|Random|RandomFloatinRange 0.0 19.0) false))
  (Components|InstancedStaticMesh|SetCustomDataValue (Variables|Default|GetInstancedStaticMesh) 0 0 (Math|Random|RandomFloatinRange 0.0 19.0) true)
  (CallFunction|LOOPMATERIALCHANGE))

(event EventBeginPlay
  ;[1 1 1] BEGIN
  (if (Variables|Default|GetRANDOMIZE)
    (CallFunction|LOOPMATERIALCHANGE)))

(event Input|KeyboardEvents|2
  (params (Key :type Key%20Structure :default "None"))
  (bind _instancedstaticmesh (Variables|Default|GetInstancedStaticMesh))
  (bind _returnvalue (Rendering|IsVisible _instancedstaticmesh))
  ;[0.5501 0.6415 1 1 32] HIDE / UNHIDE BASED ON UNIFY MATERIAL
  (:Pressed
    (Rendering|SetVisibility _instancedstaticmesh (not _returnvalue) false)
    (if _returnvalue
      (Development|PrintString "UNIFIED ISM MATERAL SHOWN" true false)
      (else
        (Development|PrintString "UNIFIED ISM  MATERAL HIDDEN" true false)))))

(fn ConstructionScript)